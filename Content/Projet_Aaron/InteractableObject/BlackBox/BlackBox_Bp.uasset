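; BlackBox_Bp is an interactable "Boîte Noire" (black box) that ends the tutorial with a scripted player death.
; Interact clears undying, flags tutorial completion and character recreation, then on press disables input and spawns a Beta_Character behind Aaron.
; A timeline turns the view around, then Beta's cry and attack animation precede damage equal to Aaron's maximum bio health.
; GetLabel shows the interest-point particles, which Tick hides every frame.
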(event EventTick
  (params (DeltaSeconds :type Float%20%28single-precision%29))
  (Rendering|SetVisibility (Variables|Default|GetInterestPointParticuleSystem) false false))

(event EventInteract
  (params (IsPressed :type Boolean) (RefToInteractActor :type Actor%20Object%20Reference))
  (bind _returnvalue (|PlayerAdvancementSubsystem))
  (Class|StatManager|SetUndying (Actor|GetComponentbyClass (Game|GetPlayerCharacter 0) "/Script/Projet_Aaron.CharacterStatManager") false)
  (Class|PlayerAdvancementSubsystem|SetCanRecreateCharacter _returnvalue true)
  (Class|PlayerAdvancementSubsystem|SetTutorialCompleted _returnvalue true)
  (if IsPressed
    (bind _asaaron_character_bp (Utilities|Casting|CastToAaronCharacterBP RefToInteractActor))
    (bind _output_get (Variables|Default|SetAaron _asaaron_character_bp))
    (Input|DisableInput _output_get (Game|GetPlayerController 0))
    (bind _returnvalue_2 (Game|SpawnActorfromClass "/Game/Projet_Aaron/Creatures/Beta/Beta_Character.Beta_Character_C" (Math|Transform|MakeTransform (+ (.location (Transformation|GetWorldTransform (Variables|/Script/Engine.Actor|GetRootComponent (Variables|Default|GetAaron)))) (* (Math|Vector|GetForwardVector (Variables|/Script/Engine.Actor|GetRootComponent (Variables|Default|GetAaron))) -2.5e+02)) (.rotation (Transformation|GetWorldTransform (Variables|/Script/Engine.Actor|GetRootComponent (Variables|Default|GetAaron)))) (.scale (Transformation|GetWorldTransform (Variables|/Script/Engine.Actor|GetRootComponent (Variables|Default|GetAaron))))) "Undefined" 0 0))
    (Variables|Default|SetBeta _returnvalue_2)
    (Variables|Default|SetInitialRotation (Transformation|GetWorldRotation (Variables|/Script/Projet_Aaron.AaronCharacter|GetFpsCamera (Variables|Default|GetAaron))))
    (Variables|Default|SetRotationToFollow (Math|Rotator|MakeRotator (- (.roll (Math|Rotator|FindLookatRotation (Transformation|GetWorldLocation (Variables|/Script/Projet_Aaron.AaronCharacter|GetFpsCamera (Variables|Default|GetAaron))) (+ (Transformation|GetWorldLocation (Variables|/Script/Projet_Aaron.AaronCharacter|GetFpsCamera (Variables|Default|GetAaron))) (* (Math|Vector|GetForwardVector (Variables|/Script/Engine.Actor|GetRootComponent (Variables|Default|GetAaron))) -1e+02)))) (.roll (Transformation|GetWorldRotation (Variables|/Script/Projet_Aaron.AaronCharacter|GetFpsCamera (Variables|Default|GetAaron))))) (- (.pitch (Math|Rotator|FindLookatRotation (Transformation|GetWorldLocation (Variables|/Script/Projet_Aaron.AaronCharacter|GetFpsCamera (Variables|Default|GetAaron))) (+ (Transformation|GetWorldLocation (Variables|/Script/Projet_Aaron.AaronCharacter|GetFpsCamera (Variables|Default|GetAaron))) (* (Math|Vector|GetForwardVector (Variables|/Script/Engine.Actor|GetRootComponent (Variables|Default|GetAaron))) -1e+02)))) (.pitch (Transformation|GetWorldRotation (Variables|/Script/Projet_Aaron.AaronCharacter|GetFpsCamera (Variables|Default|GetAaron))))) (- (.yaw (Math|Rotator|FindLookatRotation (Transformation|GetWorldLocation (Variables|/Script/Projet_Aaron.AaronCharacter|GetFpsCamera (Variables|Default|GetAaron))) (+ (Transformation|GetWorldLocation (Variables|/Script/Projet_Aaron.AaronCharacter|GetFpsCamera (Variables|Default|GetAaron))) (* (Math|Vector|GetForwardVector (Variables|/Script/Engine.Actor|GetRootComponent (Variables|Default|GetAaron))) -1e+02)))) (.yaw (Transformation|GetWorldRotation (Variables|/Script/Projet_Aaron.AaronCharacter|GetFpsCamera (Variables|Default|GetAaron)))))))
    (bind _newtrack_0 (Timeline|Timeline_0 PlayFromStart)
      (:Update
        (Pawn|SetControlRotation (Game|GetPlayerController 0) (Math|Rotator|MakeRotator (+ (.roll (* (Variables|Default|GetRotationToFollow) _newtrack_0)) (.roll (Variables|Default|GetInitialRotation))) (+ (.pitch (* (Variables|Default|GetRotationToFollow) _newtrack_0)) (.pitch (Variables|Default|GetInitialRotation))) (+ (.yaw (* (Variables|Default|GetRotationToFollow) _newtrack_0)) (.yaw (Variables|Default|GetInitialRotation))))))
      (:Finished
        (Audio|PlaySound2D "/Game/Projet_Aaron/Creatures/Beta/Assets/Sound/Beta_Cri.Beta_Cri" 1.0 1.0 0.0 0 0)
        (Utilities|FlowControl|Delay 1.0)
        (Components|Animation|PlayAnimation (Variables|/Script/Engine.Character|GetMesh (Variables|Default|GetBeta)) "/Game/Projet_Aaron/Creatures/Beta/Assets/Anim/Grosha_attack_Anim.Grosha_attack_Anim" false)
        (Utilities|FlowControl|Delay 1.0)
        (Class|StatManager|TakeDamage (Actor|GetComponentbyClass (Variables|Default|GetAaron) "/Script/Projet_Aaron.CharacterStatManager") (Class|StatManager|GetHealthBioMax (Actor|GetComponentbyClass (Variables|Default|GetAaron) "/Script/Projet_Aaron.CharacterStatManager")) 0.0)))))

(fn ConstructionScript)

(fn GetLabel
  (Rendering|SetVisibility (Variables|Default|GetInterestPointParticuleSystem) true false)
  (return "Boîte Noire"))