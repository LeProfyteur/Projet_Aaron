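; BlockingPlant is a creature obstacle that opens while a lightstick is near and closes once none remain.
; Lightstick overlaps on AffraidBoxCollision drive Open and Close, which shift the skeletal mesh vertically as a placeholder for animation.
; A looping timer calls DamageActorInTrap, which, while closed, finds actors with a StateManager component inside DamageBoxCollision.
; The attack currently only prints a debug string and applies no damage.
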(event OnComponentBeginOverlap(AffraidBoxCollision)
  (params (OverlappedComponent :type Primitive%20Component%20Object%20Reference) (OtherActor :type Actor%20Object%20Reference) (OtherComp :type Primitive%20Component%20Object%20Reference) (OtherBodyIndex :type Integer) (bFromSweep :type Boolean) (SweepResult :type Hit%20Result%20Structure%20%28by%20ref%29))
  (Utilities|Casting|CastToItem_Lightstick OtherActor)
  (CallFunction|Open))

(event OnComponentEndOverlap(AffraidBoxCollision)
  (params (OverlappedComponent :type Primitive%20Component%20Object%20Reference) (OtherActor :type Actor%20Object%20Reference) (OtherComp :type Primitive%20Component%20Object%20Reference) (OtherBodyIndex :type Integer))
  (Utilities|Casting|CastToItem_Lightstick OtherActor)
  (CallFunction|Close))

(event Custom|Check%20Damage
  (CallFunction|DamageActorinTrap))

(event EventBeginPlay
  (Utilities|Time|SetTimerbyEvent (delegate Custom|Check%20Damage) (Variables|Default|GetDelayBetweenDamage) true))

(fn ConstructionScript)

(fn Open
  (if (not (Variables|Default|GetOpenned))
    (if (not (== (Utilities|Array|Length (Collision|GetOverlappingActors (Variables|Default|GetAffraidBoxCollision) "/Game/Projet_Aaron/Item/Item_Lightstick.Item_Lightstick_C" :!class /Script/Engine.PrimitiveComponent)) 0))
      ;[1 1 1] Replace by Animation of the plant
      (Transformation|SetRelativeLocation (Variables|Default|GetSkeletalMesh) (+ (Variables|/Script/Engine.SceneComponent|GetRelativeLocation (Variables|Default|GetSkeletalMesh)) "0, 0,200.000000") false false)
      (Variables|Default|SetOpenned true))))

(fn Close
  (if (Variables|Default|GetOpenned)
    (if (== (Utilities|Array|Length (Collision|GetOverlappingActors (Variables|Default|GetAffraidBoxCollision) "/Game/Projet_Aaron/Item/Item_Lightstick.Item_Lightstick_C" :!class /Script/Engine.PrimitiveComponent)) 0)
      ;[1 1 1] Replace by Animation of the plant
      (Transformation|SetRelativeLocation (Variables|Default|GetSkeletalMesh) (+ (Variables|/Script/Engine.SceneComponent|GetRelativeLocation (Variables|Default|GetSkeletalMesh)) "0, 0,-200.000000") false false)
      (Variables|Default|SetOpenned false))))

(fn DamageActorinTrap
  (if (not (Variables|Default|GetOpenned))
    (for _array_element (Collision|GetOverlappingActors (Variables|Default|GetDamageBoxCollision) "/Script/Engine.Actor" :!class /Script/Engine.PrimitiveComponent)
      (if (!= self _array_element)
        (Utilities|IsValid (Actor|GetComponentbyClass _array_element "/Script/Projet_Aaron.StateManager")
          (:Is%20Valid
            (Development|PrintString (Utilities|String|Append "attack: " (Utilities|String|ToString(Object) _array_element)))))))))