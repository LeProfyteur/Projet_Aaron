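; Trigger volume Blueprint that plays its audio only while the player is inside it, apparently for the HUB area.
; Overlap begin and end events for player character 0 fade the Audio component in or out over a short duration.
; BeginPlay stops the audio, then fades it in if the player already overlaps the collision component, covering a spawn inside the volume.
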(event EventBeginPlay
  (bind _audio (Variables|Default|GetAudio))
  (Audio|Components|Audio|Stop _audio)
  (if (Utilities|Array|ContainsItem (Collision|GetOverlappingActors (Variables|Default|GetCollisionComponent) 0 :!class /Script/Engine.PrimitiveComponent) (Game|GetPlayerCharacter 0))
    (Audio|Components|Audio|FadeIn _audio 2.0 1.0 0.0 "Linear" :!class /Script/Engine.AudioComponent)))

(event Collision|EventActorBeginOverlap
  (params (OtherActor :type Actor%20Object%20Reference))
  (if (== OtherActor (Game|GetPlayerCharacter 0))
    (Audio|Components|Audio|FadeIn (Variables|Default|GetAudio) 2.0 1.0 0.0 "Linear" :!class /Script/Engine.AudioComponent)))

(event Collision|EventActorEndOverlap
  (params (OtherActor :type Actor%20Object%20Reference))
  (if (== OtherActor (Game|GetPlayerCharacter 0))
    (Audio|Components|Audio|FadeOut (Variables|Default|GetAudio) 2.0 0.0 "Linear" :!class /Script/Engine.AudioComponent)))

(fn ConstructionScript)