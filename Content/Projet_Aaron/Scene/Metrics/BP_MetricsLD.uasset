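; BP_MetricsLD is a level design helper actor that previews player traversal metrics as debug drawings.
; Toggling Refresh reruns the construction script, where a MultiBranch macro evaluates the Show flags for jump, grapple, jump boots and jetpack.
; Jumps use projectile path prediction from the player capsule, while grapple reach uses a forward line trace.
; The jetpack preview finds the jump arc's apex, then predicts a forward glide under overridden gravity.
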(fn ConstructionScript
  (bind _forwardarrow (Variables|Default|GetForwardArrow))
  (bind _returnvalue (Transformation|GetWorldLocation _forwardarrow))
  (if (Variables|Default|GetRefresh)
    (Variables|Default|SetRefresh false)
    (Utilities|MultiBranch (Variables|Selector|MovementSelector|GetShowJump) (Variables|Selector|TechSkills|GetShowGrapple) (Variables|Selector|TechSkills|GetShowJumpBoots) (Variables|Selector|TechSkills|GetShowJetPack)
      (:Condition1
        (Class|GameplayStatics|BlueprintPredictProjectilePathbyTraceChannel (Transformation|GetWorldLocation (Variables|Default|GetPlayerHeight)) (+ (* (Math|Vector|GetForwardVector (Variables|Default|GetForwardArrow)) (Utilities|GetSpeed)) (Variables|Private|GetJumpVelocity)) true (Variables|/Script/Engine.CapsuleComponent|GetCapsuleRadius (Variables|Default|GetPlayerHeight)) "ECC_WorldDynamic" false (Utilities|Array|MakeArray self) "ForDuration" 5.0))
      (:Condition2
        (Collision|LineTraceByChannel _returnvalue (+ _returnvalue (* (Math|Vector|GetForwardVector _forwardarrow) (Variables|Private|GetGrappleLength))) "TraceTypeQuery1" false 0 "ForDuration"))
      (:Condition3
        (Class|GameplayStatics|BlueprintPredictProjectilePathbyTraceChannel (Transformation|GetWorldLocation (Variables|Default|GetPlayerHeight)) (* (Variables|Private|GetJumpVelocity) 2.5) true (Variables|/Script/Engine.CapsuleComponent|GetCapsuleRadius (Variables|Default|GetPlayerHeight)) "ECC_WorldDynamic" false (Utilities|Array|MakeArray self) "ForDuration" 5.0))
      (:Condition4
        (bind _outpathpositions (Class|GameplayStatics|BlueprintPredictProjectilePathbyTraceChannel (Transformation|GetWorldLocation (Variables|Default|GetPlayerHeight)) (+ (* (Math|Vector|GetForwardVector (Variables|Default|GetForwardArrow)) (Utilities|GetSpeed)) (Variables|Private|GetJumpVelocity)) true (Variables|/Script/Engine.CapsuleComponent|GetCapsuleRadius (Variables|Default|GetPlayerHeight)) "ECC_WorldDynamic" false (Utilities|Array|MakeArray self) "ForDuration" 5.0))
        (bind (_array_element _array_index) (Utilities|Array|ForEachLoopwithBreak _outpathpositions :!label _label)
          (:LoopBody
            (if (not (> (.Z (Math|Vector|BreakVector _array_element)) (.z (Utilities|Array|Get(acopy) _outpathpositions (- _array_index 1)))))
              (Variables|Private|SetMaxJumpHeight _array_element)
              (Utilities|FlowControl|Sequence
                (:then_0
                  (goto _label Break))
                (:then_1
                  (Class|GameplayStatics|BlueprintPredictProjectilePathbyTraceChannel (Variables|Private|GetMaxJumpHeight) (* (Math|Vector|GetForwardVector (Variables|Default|GetForwardArrow)) (Utilities|GetSpeed)) true (Variables|/Script/Engine.CapsuleComponent|GetCapsuleRadius (Variables|Default|GetPlayerHeight)) "ECC_WorldDynamic" false (Utilities|Array|MakeArray self) "ForDuration" 5.0 15.0 2.0 -2.5e+02))))))))))