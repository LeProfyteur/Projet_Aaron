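; Poison_BP is a helper Blueprint that manually drives a poison post-processing effect from keyboard input.
; Holding A raises a poison coefficient over time and holding E lowers it, with A taking priority and the value clamped to a normalized range.
; While either key is held, Tick writes the coefficient to the Mutation scalar in the MPC_PostProcessing material parameter collection.
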(event EventTick
  (params (DeltaSeconds :type Float%20%28single-precision%29))
  (bind _returnvalue (* DeltaSeconds 0.2))
  (if (Variables|Default|GetAdding)
    (Variables|Default|SetPoisonCoef (Math|Float|Clamp(Float) (+ _returnvalue (Variables|Default|GetPoisonCoef))))
    (Rendering|Material|SetScalarParameterValue "/Game/Projet_Aaron/PostProcessingEffect/Helper/MPC_PostProcessing.MPC_PostProcessing" "Mutation" (Variables|Default|GetPoisonCoef) :!class /Script/Engine.KismetMaterialLibrary :!label _label)
    (elif (Variables|Default|GetSubtracting)
      (Variables|Default|SetPoisonCoef (Math|Float|Clamp(Float) (- (Variables|Default|GetPoisonCoef) _returnvalue)))
      (goto _label))))

(event Input|KeyboardEvents|A
  (params (Key :type Key%20Structure :default "None"))
  (:Pressed
    (Variables|Default|SetAdding true))
  (:Released
    (Variables|Default|SetAdding false)))

(event Input|KeyboardEvents|E
  (params (Key :type Key%20Structure :default "None"))
  (:Pressed
    (Variables|Default|SetSubtracting true))
  (:Released
    (Variables|Default|SetSubtracting false)))

(fn ConstructionScript)