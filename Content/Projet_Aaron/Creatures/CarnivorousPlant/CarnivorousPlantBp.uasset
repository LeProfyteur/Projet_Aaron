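; Carnivorous plant trap that bites allowed actor classes lingering inside its collision box.
; Overlaps add and remove actors in a map of time spent inside, incremented every Tick.
; Once an actor passes the player or monster time threshold, the plant plays its attack animation and damages that actor's StatManager with bio and tech damage.
; A delay timer then zeroes all timers and re-arms it; debug prints remain.
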(event OnComponentBeginOverlap(TrapCollisionBox)
  (params (OverlappedComponent :type Primitive%20Component%20Object%20Reference) (OtherActor :type Actor%20Object%20Reference) (OtherComp :type Primitive%20Component%20Object%20Reference) (OtherBodyIndex :type Integer) (bFromSweep :type Boolean) (SweepResult :type Hit%20Result%20Structure%20%28by%20ref%29))
  (for _array_element (Variables|Default|GetCanAttack)
    (if (== _array_element (Utilities|GetClass OtherActor))
      (Utilities|Map|Add (Variables|Default|GetTimeActorInTrap) OtherActor 0.0))))

(event OnComponentEndOverlap(TrapCollisionBox)
  (params (OverlappedComponent :type Primitive%20Component%20Object%20Reference) (OtherActor :type Actor%20Object%20Reference) (OtherComp :type Primitive%20Component%20Object%20Reference) (OtherBodyIndex :type Integer))
  (Utilities|Map|Remove (Variables|Default|GetTimeActorInTrap) OtherActor))

(event Custom|ResetDelayAttack
  (CallFunction|ResetAfterAttack))

(event EventTick
  (params (DeltaSeconds :type Float%20%28single-precision%29))
  (CallFunction|ShowTimeActorinTrap)
  (CallFunction|UpdateTimeActorinTrap DeltaSeconds)
  (bind _attack (CallFunction|DealDamageActorinTrap))
  (if _attack
    (Variables|Default|SetAttackReady false)
    (Utilities|Time|SetTimerbyEvent (delegate Custom|ResetDelayAttack) (Variables|Default|GetDelayBetweenAttack))))

(fn ConstructionScript)

(fn UpdateTimeActorinTrap
  (params (DeltaSecond :type Float%20%28single-precision%29))
  (bind _keys (Utilities|Map|Keys (Variables|Default|GetTimeActorInTrap)))
  (for _array_element _keys
    (Utilities|Map|Add (Variables|Default|GetTimeActorInTrap) _array_element (+ (.Value (Utilities|Map|Find (Variables|Default|GetTimeActorInTrap) _array_element)) DeltaSecond))))

(fn DealDamageActorinTrap
  (if (Variables|Default|GetAttackReady)
    (bind _keys (Utilities|Map|Keys (Variables|Default|GetTimeActorInTrap)))
    (for _array_element _keys
      (Utilities|Casting|CastToAAronCharacterCPP _array_element
        (:then
          (if (>= (.Value (Utilities|Map|Find (Variables|Default|GetTimeActorInTrap) _array_element)) (Variables|Default|GetTimeBeforeAttackPlayer))
            (CallFunction|Attack _array_element)
            (Development|PrintString "kill player")
            (return true)))
        (:CastFailed
          (if (>= (.Value (Utilities|Map|Find (Variables|Default|GetTimeActorInTrap) _array_element)) (Variables|Default|GetTimeBeforeAttackMonster))
            (CallFunction|Attack _array_element)
            (Development|PrintString "kill monster")
            (return true)))))
    (return false)
    (else
      (return false))))

(fn Attack
  (params (AttackTarget :type Actor%20Object%20Reference))
  (bind _returnvalue (Actor|GetComponentbyClass AttackTarget "/Script/Projet_Aaron.StatManager"))
  (Components|Animation|PlayAnimation (Variables|Default|GetCarnivorousPlant) "/Game/Projet_Aaron/Creatures/CarnivorousPlant/Animation/Anim_Plant_carnivore_attack_Anim.Anim_Plant_carnivore_attack_Anim" false)
  (Utilities|IsValid _returnvalue
    (:Is%20Valid
      (Class|StatManager|TakeDamage _returnvalue (Variables|Default|GetDamageBio) (Variables|Default|GetDamageTech)))))

(fn ShowTimeActorinTrap
  (bind _timeactorintrap (Variables|Default|GetTimeActorInTrap))
  (bind _keys (Utilities|Map|Keys _timeactorintrap))
  (for _array_element _keys
    (Development|PrintString (Utilities|String|ToString(Float) (.Value (Utilities|Map|Find _timeactorintrap _array_element))))))

(fn ResetAfterAttack
  (bind _keys (Utilities|Map|Keys (Variables|Default|GetTimeActorInTrap)))
  (for _array_element _keys
    (Utilities|Map|Add (Variables|Default|GetTimeActorInTrap) _array_element 0.0))
  (Variables|Default|SetAttackReady true))