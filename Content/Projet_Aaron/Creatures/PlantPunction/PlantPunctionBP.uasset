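; Harvestable plant that the player can scan and draw from with a syringe, yielding the Vie (life) syringe type.
; Its box overlap shows a French syringe-usage tip to Aaron while the plant's named metric is still zero.
; Finishing a scan increments a healing-scan metric and queues a dialog.
; GetSeringueType increments the named metric on first use, which silences the tip, and queues a follow-up dialog on every call.
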(event OnComponentBeginOverlap(Box)
  (params (OverlappedComponent :type Primitive%20Component%20Object%20Reference) (OtherActor :type Actor%20Object%20Reference) (OtherComp :type Primitive%20Component%20Object%20Reference) (OtherBodyIndex :type Integer) (bFromSweep :type Boolean) (SweepResult :type Hit%20Result%20Structure%20%28by%20ref%29))
  (Utilities|IsValid (Actor|GetComponentbyClass OtherActor "/Script/Projet_Aaron.CharacterStatManager")
    (:Is%20Valid
      (bind _returnvalue (Class|DialogSubsystem|GetMetric (Variables|Default|GetNameMetrics)))
      (if (== _returnvalue 0)
        (bind _asaaron_character_bp (Utilities|Casting|CastToAaronCharacterBP OtherActor))
        (Default|DisplayTips _asaaron_character_bp "Utilise remplis ta seringue sur cette plante avec Clic Molette (hold) pour sélectionner la seringue puis Clic Molette (rapide) pour l'utiliser")))))

(event EventBeginPlay)

(event Collision|EventActorBeginOverlap
  (params (OtherActor :type Actor%20Object%20Reference)))

(event EventTick
  (params (DeltaSeconds :type Float%20%28single-precision%29)))

(event EventScanFinished
  (Class|DialogSubsystem|IncrementMetric "Scan_soin")
  (Class|DialogSubsystem|QueueDialog "/Game/Projet_Aaron/Dialogue/DataAsset/Tutorial/2_Soin/Soin_2.Soin_2"))

(fn ConstructionScript)

(fn GetSeringueType
  (bind _namemetrics (Variables|Default|GetNameMetrics))
  (bind _returnvalue (Class|DialogSubsystem|GetMetric _namemetrics))
  (if (== _returnvalue 0)
    (Class|DialogSubsystem|IncrementMetric _namemetrics))
  (Class|DialogSubsystem|QueueDialog "/Game/Projet_Aaron/Dialogue/DataAsset/Tutorial/2_Soin/Soin_3.Soin_3")
  (return "ST_Vie"))