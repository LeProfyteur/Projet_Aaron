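; Poison plant actor that applies a poison alteration to creatures entering its sphere trigger.
; On overlap, any actor with a CreatureStatManager component receives the poison with bio damage, tech damage and mutation time parameters.
; While the named metric reads zero, an affected Aaron character also gets a French tip explaining the plant damage and the Alt-plus-direction dodge.
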(event OnComponentBeginOverlap(Sphere)
  (params (OverlappedComponent :type Primitive%20Component%20Object%20Reference) (OtherActor :type Actor%20Object%20Reference) (OtherComp :type Primitive%20Component%20Object%20Reference) (OtherBodyIndex :type Integer) (bFromSweep :type Boolean) (SweepResult :type Hit%20Result%20Structure%20%28by%20ref%29))
  (Utilities|IsValid (Actor|GetComponentbyClass OtherActor "/Script/Projet_Aaron.CreatureStatManager")
    (:Is%20Valid
      (AddComponent|AddPoisonAlteration OtherActor (Variables|Default|GetPoisonDamageBio) (Variables|Default|GetPoisonDamageTech) (Variables|Default|GetTimeMutation))
      (bind _returnvalue (Class|DialogSubsystem|GetMetric (Variables|Default|GetNameMetrics)))
      (if (== _returnvalue 0)
        (bind _asaaron_character_bp (Utilities|Casting|CastToAaronCharacterBP OtherActor))
        (Default|DisplayTips _asaaron_character_bp "Tu prend des dégâts de cette plante ! Utilise Alt et une direction pour esquiver")))))

(event EventBeginPlay)

(event Collision|EventActorBeginOverlap
  (params (OtherActor :type Actor%20Object%20Reference)))

(event EventTick
  (params (DeltaSeconds :type Float%20%28single-precision%29)))

(fn ConstructionScript)