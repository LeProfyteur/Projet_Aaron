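; BP_Tips is a world-space tutorial hint whose text differs for VR and PC players, chosen at BeginPlay by casting the player character to BP_MotionControllerCharacter.
; Each tick it yaws to face the player and checks whether the player is within MinDistance.
; When that state changes, a timeline plays or reverses to scale the tip between hidden and full size.
; The construction script previews the PC text in the editor.
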(event Custom|PlayTL
  ;[1 1 1] Play the timeline to grow ornot the tip
  (if (Variables|Default|GetIsClose)
    (bind _alpha (Timeline|TL_GrowUp Play)
      (:Update
        (Transformation|SetWorldScale3D (Variables|Default|GetDefaultSceneRoot) (Math|Vector|Lerp(Vector) "0, 0, 0" "1.000000,1.000000,1.000000" _alpha))))
    (else
      (Timeline|TL_GrowUp Reverse))))

(event EventTick
  (params (DeltaSeconds :type Float%20%28single-precision%29))
  (bind _returnvalue (Game|GetPlayerCharacter 0))
  (bind _returnvalue_2 (Transformation|GetActorLocation))
  (bind _mindistance (Variables|Default|GetMinDistance))
  (bind _returnvalue_3 (Transformation|GetActorLocation _returnvalue))
  (bind _returnvalue_4 (Math|Vector|Distance(Vector) _returnvalue_3 _returnvalue_2))
  (bind _returnvalue_5 (<= _returnvalue_4 _mindistance))
  ;[1 1 1] Check and set is close only if different, also call play tl
  (Transformation|SetActorRotation (Math|Rotator|MakeRotator 0.0 0.0 (+ (.yaw (Math|Rotator|FindLookatRotation (Transformation|GetActorLocation) (Transformation|GetActorLocation (Game|GetPlayerCharacter 0)))) 9e+01)))
  (if (not (Math|Boolean|Equal(Boolean) _returnvalue_5 (Variables|Default|GetIsClose)))
    (Variables|Default|SetIsClose _returnvalue_5)
    (CallFunction|PlayTL)))

(event EventBeginPlay
  ;[1 1 1] Check if the player is using a HMD
  (Rendering|Components|TextRender|SetText (Variables|Default|GetTipsText) (select (.bSuccess (Utilities|Casting|CastToBP_MotionControllerCharacter (Game|GetPlayerCharacter 0))) (Variables|Default|GetTipVR) (Variables|Default|GetTipPC))))

(fn ConstructionScript
  (Rendering|Components|TextRender|SetText (Variables|Default|GetTipsText) (Variables|Default|GetTipPC)))