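; Blocking plant creature that opens while lit and, when closed, damages actors caught in its trap box.
; Light events adjust a light counter to drive Open and Close, both playing the same retract animation.
; A looping timer applies bio and tech damage through each overlapping actor's StatManager.
; A tips box prompts scanning until the first scan updates a metric and removes the text component and tip.
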(event OnComponentBeginOverlap(CollisionBoxTips)
  (params (OverlappedComponent :type Primitive%20Component%20Object%20Reference) (OtherActor :type Actor%20Object%20Reference) (OtherComp :type Primitive%20Component%20Object%20Reference) (OtherBodyIndex :type Integer) (bFromSweep :type Boolean) (SweepResult :type Hit%20Result%20Structure%20%28by%20ref%29))
  (Utilities|IsValid (Actor|GetComponentbyClass OtherActor "/Script/Projet_Aaron.CharacterStatManager")
    (:Is%20Valid
      (bind _returnvalue (Class|DialogSubsystem|GetMetric (Variables|Default|GetNameMetrics)))
      (if (== _returnvalue 0)
        (bind _asaaron_character_bp (Utilities|Casting|CastToAaronCharacterBP (Game|GetPlayerCharacter 0)))
        (Default|DisplayTips _asaaron_character_bp "Tu peux scan avec T lol")))))

(event Custom|Check%20Damage
  (CallFunction|DamageActorinTrap))

(event EventBeginPlay
  (Utilities|Time|SetTimerbyEvent (delegate Custom|Check%20Damage) (Variables|Default|GetDelayBetweenDamage) true))

(event EventScanFinished
  (bind _namemetrics (Variables|Default|GetNameMetrics))
  (bind _returnvalue (Class|DialogSubsystem|GetMetric _namemetrics))
  (if (== _returnvalue 0)
    (Class|DialogSubsystem|SetMetric _namemetrics 1)
    (Components|DestroyComponent (Actor|GetComponentbyClass "/Script/Engine.TextRenderComponent"))
    (Development|PrintString "PlantScanned for the first time")
    (bind _asaaron_character_bp (Utilities|Casting|CastToAaronCharacterBP (Game|GetPlayerCharacter 0)))
    (Default|RemoveDisplayTips _asaaron_character_bp)))

(event EventLightUp
  (Math|Integer|IncrementInt (Variables|Default|GetNumberLightBy)
    (:%20%20
      (CallFunction|Open))))

(event EventTurnOff
  (bind _result (Math|Integer|DecrementInt (Variables|Default|GetNumberLightBy))
    (:%20%20
      (if (== _result 0)
        (CallFunction|Close)))))

(fn ConstructionScript)

(fn Open
  (if (not (Variables|Default|GetOpenned))
    (Components|Animation|PlayAnimation (Variables|Default|GetSkeletalMesh) "/Game/Projet_Aaron/Creatures/BlockingPlant/New_anim/Retract/Anim_plante_block_retract_Anim.Anim_plante_block_retract_Anim" false)
    (Variables|Default|SetOpenned true)))

(fn Close
  (if (Variables|Default|GetOpenned)
    (Components|Animation|PlayAnimation (Variables|Default|GetSkeletalMesh) "/Game/Projet_Aaron/Creatures/BlockingPlant/New_anim/Retract/Anim_plante_block_retract_Anim.Anim_plante_block_retract_Anim" false)
    (Variables|Default|SetOpenned false)))

(fn DamageActorinTrap
  (if (not (Variables|Default|GetOpenned))
    (for _array_element (Collision|GetOverlappingActors (Variables|Default|GetDamageBoxCollision) "/Script/Engine.Actor" :!class /Script/Engine.PrimitiveComponent)
      (if (!= self _array_element)
        (Utilities|IsValid (Actor|GetComponentbyClass _array_element "/Script/Projet_Aaron.StatManager")
          (:Is%20Valid
            (Class|StatManager|TakeDamage (Actor|GetComponentbyClass _array_element "/Script/Projet_Aaron.StatManager") (Variables|Default|GetBioDamage) (Variables|Default|GetTechDamage))))))))