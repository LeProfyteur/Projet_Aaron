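; Parent Blueprint for 3D main-menu buttons, whose click action is chosen by a ButtonType setting.
; Swap View finds a CameraActor whose display name contains CameraNameForSwap and blends the player's view to it.
; Play in VR and Play in PC both open the tutorial level, while Quitter quits the game.
; The construction script writes the configured Texte into the button's TextRender.
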(event EventClicked
  (switch Utilities|FlowControl|Switch|SwitchonE_ButtonType (Variables|Default|GetButtonType)
    (:NewEnumerator0
      (bind _outactors (Actor|GetAllActorsOfClass "/Script/Engine.CameraActor"))
      (bind _array_element (Utilities|Array|ForEachLoopwithBreak _outactors :!label _label)
        (:LoopBody
          (if (Utilities|String|Contains (Utilities|GetDisplayName _array_element) (Variables|Default|GetCameraNameForSwap))
            (Utilities|FlowControl|Sequence
              (:then_0
                (goto _label Break))
              (:then_1
                (Game|Player|SetViewTargetwithBlend (Game|GetPlayerController 0) _array_element 0.5 "VTBlend_Linear" 0.0 false)))))))
    (:NewEnumerator3
      (Game|OpenLevel(byName) "Lvl_Tutoriel" :!label _label_2))
    (:NewEnumerator4
      (goto _label_2))
    (:NewEnumerator6
      (Game|QuitGame 0 "Quit" false))))

(fn ConstructionScript
  (Rendering|Components|TextRender|SetText (Variables|Default|GetTextRender) (Variables|Default|GetTexte)))