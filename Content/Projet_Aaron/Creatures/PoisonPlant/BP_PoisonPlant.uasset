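; BP_PoisonPlant is a scannable poisonous plant ("Raflesiata") that poisons creatures lingering in its trigger sphere.
; Overlap activates particles and starts a one-second dodge window, then poisons the last entrant if still inside, with a CreatureStatManager and unpoisoned.
; A metric check gates first-time poisoning dialogs and the player's dodge tip, while scanning queues dialogs and records the entry.
; The construction script selects one of four meshes, randomly or by ID.
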(event OnComponentBeginOverlap(Sphere)
  (params (OverlappedComponent :type Primitive%20Component%20Object%20Reference) (OtherActor :type Actor%20Object%20Reference) (OtherComp :type Primitive%20Component%20Object%20Reference) (OtherBodyIndex :type Integer) (bFromSweep :type Boolean) (SweepResult :type Hit%20Result%20Structure%20%28by%20ref%29))
  (Utilities|Time|SetTimerbyEvent (delegate Custom|PlayerStayed) 1.0) ; To let the player time to dodge
  (Variables|Default|SetOverlapedActor OtherActor)
  (Components|Activation|Activate (Variables|Default|GetParticleSystem) true))

(event Custom|PlayerStayed
  (bind _overlapedactor (Variables|Default|GetOverlapedActor))
  (bind _returnvalue (Actor|GetComponentbyClass _overlapedactor "/Script/Projet_Aaron.CreatureStatManager"))
  (if (Utilities|Array|ContainsItem (Collision|GetOverlappingActors (Variables|Default|GetSphere) 0 :!class /Script/Engine.PrimitiveComponent) _overlapedactor)
    (Utilities|IsValid _returnvalue
      (:Is%20Valid
        (if (not (Class|CreatureStatManager|GetPoisonAlteration _returnvalue))
          (AddComponent|AddPoisonAlteration _overlapedactor (Variables|Default|GetPoisonDamageBio) (Variables|Default|GetPoisonDamageTech) (Variables|Default|GetTimeMutation))
          (bind _returnvalue_2 (Class|DialogSubsystem|GetMetric (Variables|Default|GetNameMetrics)))
          (if (== _returnvalue_2 0)
            (bind _asaaron_character_bp (Utilities|Casting|CastToAaronCharacterBP _overlapedactor))
            (Class|DialogSubsystem|IncrementMetric "Poisonned_trigger")
            (Class|DialogSubsystem|QueueDialog "/Game/Projet_Aaron/Dialogue/DataAsset/Tutorial/Poison_plante/Poisonned_Before_Scan.Poisonned_Before_Scan")
            (Class|DialogSubsystem|QueueDialog "/Game/Projet_Aaron/Dialogue/DataAsset/Tutorial/Poison_plante/Poisonned_After_Scan.Poisonned_After_Scan")
            (Default|DisplayTips _asaaron_character_bp "PoisonPlant" "Dodge" "None")))))))

(event EventScanFinished
  (Class|DialogSubsystem|QueueDialog "/Game/Projet_Aaron/Dialogue/DataAsset/Tutorial/Poison_plante/Scan_Before_Poisonned.Scan_Before_Poisonned")
  (Class|DialogSubsystem|QueueDialog "/Game/Projet_Aaron/Dialogue/DataAsset/Tutorial/Poison_plante/Scan_After_Poisonned.Scan_After_Poisonned")
  (Class|PlayerAdvancementSubsystem|SetScannableItemStatus "PoisonPlantScan" true))

(fn ConstructionScript
  (bind _staticmeshcomponent (Variables|Debug|GetStaticMeshComponent))
  (if (Variables|Default|GetGenerateAleatoireMeshModel)
    (Variables|Default|SetGenerateAleatoireMeshModel false)
    (Variables|Default|SetIndexModel (Math|Random|RandomIntegerinRange 0 3))
    (else
      (Variables|Default|SetIndexModel (- (Variables|Default|GetPlanteMeshID) 1))))
  (switch int (Variables|Default|GetIndexModel)
    (:Default
      (Components|StaticMesh|SetStaticMesh _staticmeshcomponent "/Game/Projet_Aaron/Props/Props_I3D/Végétation_Passive/Atlas_plants_multiples/Plants_3_Raflesiata.Plants_3_Raflesiata" :!label _label))
    (:0
      (goto _label))
    (:1
      (Components|StaticMesh|SetStaticMesh _staticmeshcomponent "/Game/Projet_Aaron/Props/Props_I3D/Végétation_Passive/Atlas_plant_3/Plant_slot_1_variations_polySurface38.Plant_slot_1_variations_polySurface38"))
    (:2
      (Components|StaticMesh|SetStaticMesh _staticmeshcomponent "/Game/Projet_Aaron/Props/Props_I3D/Végétation_Passive/Atlas_plant_3/Plant_slot_1_variations_polySurface49.Plant_slot_1_variations_polySurface49"))
    (:3
      (Components|StaticMesh|SetStaticMesh _staticmeshcomponent "/Game/Projet_Aaron/Props/Props_I3D/Végétation_Passive/Atlas_plant_3/Plant_slot_1_variations_polySurface50.Plant_slot_1_variations_polySurface50"))))

(fn GetLabel
  (return "Raflesiata"))